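; BP_Case is a typed tile actor, apparently a board square, with start (DEPART), finish (FIN) and four color types.
; ChangeType maps the MType value to a colored material for the InternCircle component.
; That material is applied on BeginPlay and reapplied every Tick, so the circle follows any runtime change to MType.
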(event `self.ReceiveBeginPlay`
  (bind _meterial (`self.ChangeType` (`self.m_type`)))
  (`PrimitiveComponent.SetMaterial` (`self.internCircle`) 0 _meterial))

(event `self.ReceiveActorBeginOverlap`
  (params (OtherActor :type "Actor Object Reference")))

(event `self.ReceiveTick`
  (params (DeltaSeconds :type "Float (single-precision)"))
  (bind _meterial (`self.ChangeType` (`self.m_type`)))
  (`PrimitiveComponent.SetMaterial` (`self.internCircle`) 0 _meterial))

(fn `ChangeType`
  (params (type :type "/Game/BluePrints/Enums/EType Enum"))
  (returns (Meterial :type "Material Object Reference"))
  (switch `/Game/BluePrints/Enums/EType` type
    (:`NewEnumerator0`
      (return "/Game/Materials/Purple.Purple"))
    (:`NewEnumerator1`
      (return "/Game/Materials/Black.Black"))
    (:`NewEnumerator2`
      (return "/Game/Materials/Blue.Blue"))
    (:`NewEnumerator3`
      (return "/Game/Materials/Green.Green"))
    (:`NewEnumerator4`
      (return "/Game/Materials/Red.Red"))
    (:`NewEnumerator5`
      (return "/Game/Materials/Yellow.Yellow"))))

(fn `UserConstructionScript`)