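; Pawn for the color level, representing a player with one of four colors shown as a costume material on its skeletal mesh.
; The material is applied from PlayerColor on BeginPlay and again whenever SetColor changes it.
; Tick caches the actor location as CurrentPosition, while Move instantly relocates the pawn in X/Y, keeping Z and syncing NextPosition.
; Accessors expose color, current and next positions, and a NbColor value.
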(event `self.ReceiveBeginPlay`
  (bind _skeletalmesh (`self.SkeletalMesh`))
  (switch `/Game/BluePrints/Enums/BP_EType` (`self.playerColor`)
    (:`NewEnumerator2`
      (`PrimitiveComponent.SetMaterial` _skeletalmesh 0 "/Game/Materials/Captain/cosutumeBlue.cosutumeBlue"))
    (:`NewEnumerator3`
      (`PrimitiveComponent.SetMaterial` _skeletalmesh 0 "/Game/Materials/Captain/costumeGreen.costumeGreen"))
    (:`NewEnumerator4`
      (`PrimitiveComponent.SetMaterial` _skeletalmesh 0 "/Game/Materials/Captain/costumeRed.costumeRed"))
    (:`NewEnumerator5`
      (`PrimitiveComponent.SetMaterial` _skeletalmesh 0 "/Game/Materials/Captain/cosutumeYellow.cosutumeYellow")))
  (set `self.nextPosition` (`self.currentPosition`)))

(event `self.ReceiveActorBeginOverlap`
  (params (OtherActor :type "Actor Object Reference")))

(event `self.ReceiveTick`
  (params (DeltaSeconds :type "Float (single-precision)"))
  (set `self.currentPosition` (`self.K2_GetActorLocation`)))

(fn `GetColor`
  (returns (color :type "/Game/BluePrints/Enums/BP_EType Enum"))
  (return (`self.playerColor`)))

(fn `GetCurrentPos`
  (returns (position :type "Vector Structure"))
  (return (`self.currentPosition`)))

(fn `GetNbColor`
  (returns (nb :type Integer))
  (return (`self.nbColor`)))

(fn `GetNextPos`
  (returns (position :type "Vector Structure"))
  (return (`self.nextPosition`)))

(fn `Move`
  (params (position :type "Vector Structure"))
  (bind (_currentposition_x _currentposition_y _currentposition_z) (`KismetMathLibrary.BreakVector` (`self.currentPosition`)))
  (bind _output_get (set `self.currentPosition` (`KismetMathLibrary.MakeVector` position_X position_Y _currentposition_z)))
  (bind _output_get_2 (set `self.nextPosition` _output_get))
  (`self.K2_SetActorLocation` _output_get_2))

(fn `SetColor`
  (params (color :type "/Game/BluePrints/Enums/BP_EType Enum"))
  (bind _skeletalmesh (`self.SkeletalMesh`))
  (bind _output_get (set `self.playerColor` color))
  (switch `/Game/BluePrints/Enums/BP_EType` _output_get
    (:`NewEnumerator2`
      (`PrimitiveComponent.SetMaterial` _skeletalmesh 0 "/Game/Materials/Captain/cosutumeBlue.cosutumeBlue"))
    (:`NewEnumerator3`
      (`PrimitiveComponent.SetMaterial` _skeletalmesh 0 "/Game/Materials/Captain/costumeGreen.costumeGreen"))
    (:`NewEnumerator4`
      (`PrimitiveComponent.SetMaterial` _skeletalmesh 0 "/Game/Materials/Captain/costumeRed.costumeRed"))
    (:`NewEnumerator5`
      (`PrimitiveComponent.SetMaterial` _skeletalmesh 0 "/Game/Materials/Captain/cosutumeYellow.cosutumeYellow"))))

(fn `SetCurrentPos`
  (params (position :type "Vector Structure"))
  (set `self.currentPosition` position))

(fn `SetNbColor`
  (params (nb :type Integer))
  (set `self.nbColor` nb))

(fn `SetNextPos`
  (params (position :type "Vector Structure"))
  (set `self.nextPosition` position))

(fn `UserConstructionScript`)