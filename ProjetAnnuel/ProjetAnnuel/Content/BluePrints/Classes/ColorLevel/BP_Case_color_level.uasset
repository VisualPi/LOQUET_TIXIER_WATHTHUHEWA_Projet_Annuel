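; BP_Case_color_level is a tile for the color level that takes on the color of the player pawn that hits it.
; Hits on InternCircle or Collider read the color from BP_Pawn_Color_Level and store it in MType, with no guard on the tile's current type.
; ChangeType maps MType (start, finish, colors or default) to an InternCircle material, reapplied on BeginPlay and every Tick.
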(event `/Game/BluePrints/Classes/BP_Case.ReceiveBeginPlay`
  (`self.ChangeType` (`self.m_type`)))

(event `self.ReceiveActorBeginOverlap`
  (params (OtherActor :type "Actor Object Reference")))

(event `/Game/BluePrints/Classes/BP_Case.ReceiveTick`
  (params (DeltaSeconds :type "Float (single-precision)"))
  (`self.ChangeType` (`self.m_type`)))

(event `self.internCircle.OnComponentHit`
  (params (OtherActor :type "Actor Object Reference") (OtherComp :type "PrimitiveComponent Object Reference") (NormalImpulse :type "Vector Structure") (Hit :type "HitResult Structure (by ref)"))
  (`self.ChangeTypeFromCollision` OtherActor))

(event `self.collider.OnComponentHit`
  (params (OtherActor :type "Actor Object Reference") (OtherComp :type "PrimitiveComponent Object Reference") (NormalImpulse :type "Vector Structure") (Hit :type "HitResult Structure (by ref)"))
  (`self.ChangeTypeFromCollision` OtherActor))

(fn `ChangeType`
  (params (type :type "/Game/BluePrints/Enums/BP_EType Enum"))
  (switch `/Game/BluePrints/Enums/BP_EType` type
    (:`NewEnumerator0`
      (`PrimitiveComponent.SetMaterial` (`self.internCircle`) 0 "/Game/Materials/Purple.Purple")
      (set `self.m_type` "NewEnumerator0"))
    (:`NewEnumerator1`
      (`PrimitiveComponent.SetMaterial` (`self.internCircle`) 0 "/Game/Materials/Black.Black")
      (set `self.m_type` "NewEnumerator1"))
    (:`NewEnumerator2`
      (`PrimitiveComponent.SetMaterial` (`self.internCircle`) 0 "/Game/Materials/Blue.Blue")
      (set `self.m_type` "NewEnumerator2"))
    (:`NewEnumerator3`
      (`PrimitiveComponent.SetMaterial` (`self.internCircle`) 0 "/Game/Materials/Green.Green")
      (set `self.m_type` "NewEnumerator3"))
    (:`NewEnumerator4`
      (`PrimitiveComponent.SetMaterial` (`self.internCircle`) 0 "/Game/Materials/Red.Red")
      (set `self.m_type` "NewEnumerator4"))
    (:`NewEnumerator5`
      (`PrimitiveComponent.SetMaterial` (`self.internCircle`) 0 "/Game/Materials/Yellow.Yellow")
      (set `self.m_type` "NewEnumerator5"))
    (:`NewEnumerator7`
      (`PrimitiveComponent.SetMaterial` (`self.internCircle`) 0 "/Game/Materials/White.White")
      (set `self.m_type` "NewEnumerator7"))))

(fn `ChangeTypeFromCollision`
  (params (collidedActor :type "Actor Object Reference"))
  (bind _output_get (set `self.collidedActor` collidedActor))
  (if (== "/Game/BluePrints/Classes/ColorLevel/BP_Pawn_Color_Level.BP_Pawn_Color_Level_C" (`GameplayStatics.GetObjectClass` _output_get))
    (bind _asbp_pawn_color_level (cast `/Game/BluePrints/Classes/ColorLevel/BP_Pawn_Color_Level` (`self.collidedActor`))
      (:`then`
        (set `self.playerBP` _asbp_pawn_color_level)
        (bind _color (`/Game/BluePrints/Classes/ColorLevel/BP_Pawn_Color_Level.GetColor` (`self.playerBP`)))
        (set `self.m_type` _color))
      (:`CastFailed`
        _)))
  (return))

(fn `UserConstructionScript`)