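; Player controller for the Color Level that handles grid-style movement input for up to four local players.
; Each player has separate move actions, which look up that player's BP_Pawn_Color_Level by controller index rather than using this controller's own pawn.
; A press sets the pawn's next position 200 units from its current one along X or Y.
; An IsHuman flag has a getter and setter; when false, Tick only prints an AI message once.
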(event `self.ReceiveBeginPlay`)

(event `self.ReceiveTick`
  (params (DeltaSeconds :type "Float (single-precision)"))
  (if (not (`self.isHuman`))
    (`/Engine/EditorBlueprintResources/StandardMacros.DoOnce` false
      (:`Completed`
        (`KismetSystemLibrary.PrintString` "playing as AI")))))

(event `InputAction|moveRight_P0`
  (params (Key :type "Key Structure" :default "AnyKey"))
  ;[1 1 1] Inputs mouvement P0
  (:`Pressed`
    (bind _asbp_pawn_color_level (cast `/Game/BluePrints/Classes/ColorLevel/BP_Pawn_Color_Level` (`self.K2_GetPawn` (`GameplayStatics.GetPlayerController` 0))))
    (bind _position (`/Game/BluePrints/Classes/ColorLevel/BP_Pawn_Color_Level.GetCurrentPos` _asbp_pawn_color_level))
    (`/Game/BluePrints/Classes/ColorLevel/BP_Pawn_Color_Level.SetNextPos` _asbp_pawn_color_level (`KismetMathLibrary.MakeVector` (+ (.x _position) 200.0) (.y _position) (.z _position)))))

(event `InputAction|moveRight_P1`
  (params (Key :type "Key Structure" :default "AnyKey"))
  ;[1 1 1] Inputs mouvement P1
  (:`Pressed`
    (bind _asbp_pawn_color_level (cast `/Game/BluePrints/Classes/ColorLevel/BP_Pawn_Color_Level` (`self.K2_GetPawn` (`GameplayStatics.GetPlayerController` 1))))
    (bind _position (`/Game/BluePrints/Classes/ColorLevel/BP_Pawn_Color_Level.GetCurrentPos` _asbp_pawn_color_level))
    (`/Game/BluePrints/Classes/ColorLevel/BP_Pawn_Color_Level.SetNextPos` _asbp_pawn_color_level (`KismetMathLibrary.MakeVector` (+ (.x _position) 200.0) (.y _position) (.z _position)))))

(event `InputAction|moveLeft_P0`
  (params (Key :type "Key Structure" :default "AnyKey"))
  ;[1 1 1] Inputs mouvement P0
  (:`Pressed`
    (bind _asbp_pawn_color_level (cast `/Game/BluePrints/Classes/ColorLevel/BP_Pawn_Color_Level` (`self.K2_GetPawn` (`GameplayStatics.GetPlayerController` 0))))
    (bind _position (`/Game/BluePrints/Classes/ColorLevel/BP_Pawn_Color_Level.GetCurrentPos` _asbp_pawn_color_level))
    (`/Game/BluePrints/Classes/ColorLevel/BP_Pawn_Color_Level.SetNextPos` _asbp_pawn_color_level (`KismetMathLibrary.MakeVector` (- (.x _position) 200.0) (.y _position) (.z _position)))))

(event `InputAction|moveLeft_P1`
  (params (Key :type "Key Structure" :default "AnyKey"))
  ;[1 1 1] Inputs mouvement P1
  (:`Pressed`
    (bind _asbp_pawn_color_level (cast `/Game/BluePrints/Classes/ColorLevel/BP_Pawn_Color_Level` (`self.K2_GetPawn` (`GameplayStatics.GetPlayerController` 1))))
    (bind _position (`/Game/BluePrints/Classes/ColorLevel/BP_Pawn_Color_Level.GetCurrentPos` _asbp_pawn_color_level))
    (`/Game/BluePrints/Classes/ColorLevel/BP_Pawn_Color_Level.SetNextPos` _asbp_pawn_color_level (`KismetMathLibrary.MakeVector` (- (.x _position) 200.0) (.y _position) (.z _position)))))

(event `InputAction|moveDown_P0`
  (params (Key :type "Key Structure" :default "AnyKey"))
  ;[1 1 1] Inputs mouvement P0
  (:`Pressed`
    (bind _asbp_pawn_color_level (cast `/Game/BluePrints/Classes/ColorLevel/BP_Pawn_Color_Level` (`self.K2_GetPawn` (`GameplayStatics.GetPlayerController` 0))))
    (bind _position (`/Game/BluePrints/Classes/ColorLevel/BP_Pawn_Color_Level.GetCurrentPos` _asbp_pawn_color_level))
    (`/Game/BluePrints/Classes/ColorLevel/BP_Pawn_Color_Level.SetNextPos` _asbp_pawn_color_level (`KismetMathLibrary.MakeVector` (.x _position) (+ (.y _position) 200.0) (.z _position)))))

(event `InputAction|moveDown_P1`
  (params (Key :type "Key Structure" :default "AnyKey"))
  ;[1 1 1] Inputs mouvement P1
  (:`Pressed`
    (bind _asbp_pawn_color_level (cast `/Game/BluePrints/Classes/ColorLevel/BP_Pawn_Color_Level` (`self.K2_GetPawn` (`GameplayStatics.GetPlayerController` 1))))
    (bind _position (`/Game/BluePrints/Classes/ColorLevel/BP_Pawn_Color_Level.GetCurrentPos` _asbp_pawn_color_level))
    (`/Game/BluePrints/Classes/ColorLevel/BP_Pawn_Color_Level.SetNextPos` _asbp_pawn_color_level (`KismetMathLibrary.MakeVector` (.x _position) (+ (.y _position) 200.0) (.z _position)))))

(event `InputAction|moveUp_P0`
  (params (Key :type "Key Structure" :default "AnyKey"))
  ;[1 1 1] Inputs mouvement P0
  (:`Pressed`
    (bind _asbp_pawn_color_level (cast `/Game/BluePrints/Classes/ColorLevel/BP_Pawn_Color_Level` (`self.K2_GetPawn` (`GameplayStatics.GetPlayerController` 0))))
    (bind _position (`/Game/BluePrints/Classes/ColorLevel/BP_Pawn_Color_Level.GetCurrentPos` _asbp_pawn_color_level))
    (`/Game/BluePrints/Classes/ColorLevel/BP_Pawn_Color_Level.SetNextPos` _asbp_pawn_color_level (`KismetMathLibrary.MakeVector` (.x _position) (- (.y _position) 200.0) (.z _position)))))

(event `InputAction|moveUp_P1`
  (params (Key :type "Key Structure" :default "AnyKey"))
  ;[1 1 1] Inputs mouvement P1
  (:`Pressed`
    (bind _asbp_pawn_color_level (cast `/Game/BluePrints/Classes/ColorLevel/BP_Pawn_Color_Level` (`self.K2_GetPawn` (`GameplayStatics.GetPlayerController` 1))))
    (bind _position (`/Game/BluePrints/Classes/ColorLevel/BP_Pawn_Color_Level.GetCurrentPos` _asbp_pawn_color_level))
    (`/Game/BluePrints/Classes/ColorLevel/BP_Pawn_Color_Level.SetNextPos` _asbp_pawn_color_level (`KismetMathLibrary.MakeVector` (.x _position) (- (.y _position) 200.0) (.z _position)))))

(event `InputAction|moveRight_P2`
  (params (Key :type "Key Structure" :default "AnyKey"))
  ;[1 1 1] Inputs mouvement P2
  (:`Pressed`
    (bind _asbp_pawn_color_level (cast `/Game/BluePrints/Classes/ColorLevel/BP_Pawn_Color_Level` (`self.K2_GetPawn` (`GameplayStatics.GetPlayerController` 2))))
    (bind _position (`/Game/BluePrints/Classes/ColorLevel/BP_Pawn_Color_Level.GetCurrentPos` _asbp_pawn_color_level))
    (`/Game/BluePrints/Classes/ColorLevel/BP_Pawn_Color_Level.SetNextPos` _asbp_pawn_color_level (`KismetMathLibrary.MakeVector` (+ (.x _position) 200.0) (.y _position) (.z _position)))))

(event `InputAction|moveRight_P3`
  (params (Key :type "Key Structure" :default "AnyKey"))
  ;[1 1 1] Inputs mouvement P3
  (:`Pressed`
    (bind _asbp_pawn_color_level (cast `/Game/BluePrints/Classes/ColorLevel/BP_Pawn_Color_Level` (`self.K2_GetPawn` (`GameplayStatics.GetPlayerController` 3))))
    (bind _position (`/Game/BluePrints/Classes/ColorLevel/BP_Pawn_Color_Level.GetCurrentPos` _asbp_pawn_color_level))
    (`/Game/BluePrints/Classes/ColorLevel/BP_Pawn_Color_Level.SetNextPos` _asbp_pawn_color_level (`KismetMathLibrary.MakeVector` (+ (.x _position) 200.0) (.y _position) (.z _position)))))

(event `InputAction|moveLeft_P2`
  (params (Key :type "Key Structure" :default "AnyKey"))
  ;[1 1 1] Inputs mouvement P2
  (:`Pressed`
    (bind _asbp_pawn_color_level (cast `/Game/BluePrints/Classes/ColorLevel/BP_Pawn_Color_Level` (`self.K2_GetPawn` (`GameplayStatics.GetPlayerController` 2))))
    (bind _position (`/Game/BluePrints/Classes/ColorLevel/BP_Pawn_Color_Level.GetCurrentPos` _asbp_pawn_color_level))
    (`/Game/BluePrints/Classes/ColorLevel/BP_Pawn_Color_Level.SetNextPos` _asbp_pawn_color_level (`KismetMathLibrary.MakeVector` (- (.x _position) 200.0) (.y _position) (.z _position)))))

(event `InputAction|moveLeft_P3`
  (params (Key :type "Key Structure" :default "AnyKey"))
  ;[1 1 1] Inputs mouvement P3
  (:`Pressed`
    (bind _asbp_pawn_color_level (cast `/Game/BluePrints/Classes/ColorLevel/BP_Pawn_Color_Level` (`self.K2_GetPawn` (`GameplayStatics.GetPlayerController` 3))))
    (bind _position (`/Game/BluePrints/Classes/ColorLevel/BP_Pawn_Color_Level.GetCurrentPos` _asbp_pawn_color_level))
    (`/Game/BluePrints/Classes/ColorLevel/BP_Pawn_Color_Level.SetNextPos` _asbp_pawn_color_level (`KismetMathLibrary.MakeVector` (- (.x _position) 200.0) (.y _position) (.z _position)))))

(event `InputAction|moveDown_P2`
  (params (Key :type "Key Structure" :default "AnyKey"))
  ;[1 1 1] Inputs mouvement P2
  (:`Pressed`
    (bind _asbp_pawn_color_level (cast `/Game/BluePrints/Classes/ColorLevel/BP_Pawn_Color_Level` (`self.K2_GetPawn` (`GameplayStatics.GetPlayerController` 2))))
    (bind _position (`/Game/BluePrints/Classes/ColorLevel/BP_Pawn_Color_Level.GetCurrentPos` _asbp_pawn_color_level))
    (`/Game/BluePrints/Classes/ColorLevel/BP_Pawn_Color_Level.SetNextPos` _asbp_pawn_color_level (`KismetMathLibrary.MakeVector` (.x _position) (+ (.y _position) 200.0) (.z _position)))))

(event `InputAction|moveDown_P3`
  (params (Key :type "Key Structure" :default "AnyKey"))
  ;[1 1 1] Inputs mouvement P3
  (:`Pressed`
    (bind _asbp_pawn_color_level (cast `/Game/BluePrints/Classes/ColorLevel/BP_Pawn_Color_Level` (`self.K2_GetPawn` (`GameplayStatics.GetPlayerController` 3))))
    (bind _position (`/Game/BluePrints/Classes/ColorLevel/BP_Pawn_Color_Level.GetCurrentPos` _asbp_pawn_color_level))
    (`/Game/BluePrints/Classes/ColorLevel/BP_Pawn_Color_Level.SetNextPos` _asbp_pawn_color_level (`KismetMathLibrary.MakeVector` (.x _position) (+ (.y _position) 200.0) (.z _position)))))

(event `InputAction|moveUp_P2`
  (params (Key :type "Key Structure" :default "AnyKey"))
  ;[1 1 1] Inputs mouvement P2
  (:`Pressed`
    (bind _asbp_pawn_color_level (cast `/Game/BluePrints/Classes/ColorLevel/BP_Pawn_Color_Level` (`self.K2_GetPawn` (`GameplayStatics.GetPlayerController` 2))))
    (bind _position (`/Game/BluePrints/Classes/ColorLevel/BP_Pawn_Color_Level.GetCurrentPos` _asbp_pawn_color_level))
    (`/Game/BluePrints/Classes/ColorLevel/BP_Pawn_Color_Level.SetNextPos` _asbp_pawn_color_level (`KismetMathLibrary.MakeVector` (.x _position) (- (.y _position) 200.0) (.z _position)))))

(event `InputAction|moveUp_P3`
  (params (Key :type "Key Structure" :default "AnyKey"))
  ;[1 1 1] Inputs mouvement P3
  (:`Pressed`
    (bind _asbp_pawn_color_level (cast `/Game/BluePrints/Classes/ColorLevel/BP_Pawn_Color_Level` (`self.K2_GetPawn` (`GameplayStatics.GetPlayerController` 3))))
    (bind _position (`/Game/BluePrints/Classes/ColorLevel/BP_Pawn_Color_Level.GetCurrentPos` _asbp_pawn_color_level))
    (`/Game/BluePrints/Classes/ColorLevel/BP_Pawn_Color_Level.SetNextPos` _asbp_pawn_color_level (`KismetMathLibrary.MakeVector` (.x _position) (- (.y _position) 200.0) (.z _position)))))

(fn `GetIsHuman`
  (returns (isHuman :type Boolean))
  (return (`self.isHuman`)))

(fn `SetIsHuman`
  (params (isHuman :type Boolean))
  (set `self.isHuman` isHuman))

(fn `UserConstructionScript`)